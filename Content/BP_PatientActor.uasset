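; Patient actor that simulates swapping patients by sliding out, changing appearance and sliding back in from the opposite side.
; RequestPatientSwap, also bound to debug key I, starts a Tick-driven exit, enter and standby state machine, rejecting requests mid-swap.
; Past MaxLangth, the actor jumps across its start point, randomizes head mesh visibility and eye, mouth and nose materials, then returns until nearly at the start.
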(event EventBeginPlay
  ;[1 1 1] Initialize
  (Variables|Default|SetchangeOrder false)
  (Variables|Default|SetfirstPos (.Location (Math|Transform|BreakTransform (Transformation|GetActorTransform))))
  (Variables|Default|SetpatientReplacementStatus 0)
  (Variables|Default|SetbEnablePatientSwap true)
  (CallFunction|RandomlyChangestheMaterial -1))

(event EventTick
  (params (DeltaSeconds :type Float%20%28single-precision%29))
  (bind _returnvalue (Transformation|GetActorLocation))
  (bind _speed (Variables|Default|Getspeed))
  (bind _directionoftravel (Variables|Default|GetdirectionOfTravel))
  (bind _firstpos (Variables|Default|GetfirstPos))
  (bind _returnvalue_2 (Math|Rotator|MakeRotator 0.0 0.0 _directionoftravel))
  (bind _returnvalue_3 (- _returnvalue _firstpos))
  (bind _returnvalue_4 (Math|Vector|VectorLength _returnvalue_3))
  (bind _returnvalue_5 (Math|Vector|GetRightVector _returnvalue_2))
  (bind _returnvalue_6 (Math|Vector|VectorLength _returnvalue_3))
  (bind _returnvalue_7 (* _returnvalue_5 _speed))
  (bind _returnvalue_8 (Math|Conversions|ToTransform(Vector) _returnvalue_7))
  ;[1 1 1] Update
  ;;[1 1 1] Early return when no patient replacement order was issued.
  (if (Variables|Default|GetchangeOrder)
    ;;[1 1 1] Change the processing content depending on the state.
    (switch int (Variables|Default|GetpatientReplacementStatus)
      (:0
        ;;[1 1 1] "StandBy" Processing
        (Variables|Default|SetbEnablePatientSwap true)
        (Variables|Default|SetchangeOrder false))
      (:1
        ;;[1 1 1] "PatientExit" Processing
        ;;;[1 1 1] Exit move Processing
        (Class|Actor|AddActorLocalTransform _returnvalue_8 false false)
        (Variables|Default|Setlangth _returnvalue_6) ; Debugging process to check the distance diffrence from the initial position.
        ;;;[1 1 1] Determine if this have strayed too far from your initial location
        (if (> _returnvalue_6 (Variables|Default|GetmaxLangth))
          ;;;[1 1 1] Position the patient for entry.
          (Class|Actor|AddActorLocalTransform (Math|Conversions|ToTransform(Vector) (* _returnvalue_3 (* 1.0 -2.0))) false false)
          (Variables|Default|SetpatientReplacementStatus 2) ; Set status to "PatientEntering".
          (CallFunction|RandomlyChangestheMaterial -1)
          (CallFunction|UpdateFacePart true)))
      (:2
        ;;[1 1 1] "PatientEntering" Processing
        ;;;[1 1 1] Enter move Processing
        (Class|Actor|AddActorLocalTransform _returnvalue_8 false false)
        (Variables|Default|Setlangth _returnvalue_4) ; Debugging process to check the distance diffrence from the initial position.
        ;;;[1 1 1] Determine if this have strayed too far from your initial location
        (if (< _returnvalue_4 0.1)
          (Variables|Default|SetpatientReplacementStatus 0) ; Set status to "StandBy".
        )))))

(event Input|KeyboardEvents|DebugKeyI
  (params (Key :type Key%20Structure :default "None") (ActionValue :type Input%20Action%20Value%20Structure))
  ;[1 1 1] Debug function to instruct patient swapping
  (:Pressed
    (CallFunction|RequestPatientSwap)))

(fn ConstructionScript)

(fn RequestPatientSwap
  (if (Variables|Default|GetbEnablePatientSwap)
    (Variables|Default|SetchangeOrder true)
    (Variables|Default|SetbEnablePatientSwap false) ; Disable patient admission.
    (Variables|Default|SetpatientReplacementStatus 1) ; Set status to "PatientExit".
    (else
      (Development|PrintString "Patient swap request was rejected: FirstProgramActor is not accepting swap orders at the moment."))))

(fn RandomlyChangestheMaterial
  (params (selectMaterialNum :type Integer))
  ;[1 1 1] Branch when the value is -1(default).
  (if (< selectMaterialNum 0)
    ;[1 1 1] Get a random value and save it to nowHead.
    (Variables|Default|SetnowHead (Math|Random|RandomInteger (Variables|Default|GetmaxMaterialVolume)))
    (else
      (Variables|Default|SetnowHead selectMaterialNum) ; Save the arguments to nowHead.
    ))
  ;[1 1 1] Display the head part corresponding to the value in nowHead.
  (Rendering|SetVisibility (Variables|Default|GetheadPartA) (== (Variables|Default|GetnowHead) 0) false)
  (Rendering|SetVisibility (Variables|Default|GetheadPartB) (== (Variables|Default|GetnowHead) 1) false)
  (Rendering|SetVisibility (Variables|Default|GetheadPartC) (== (Variables|Default|GetnowHead) 2) false))

(fn UpdateFacePart
  (params (bRandomize :type Boolean) (eye :type Integer) (mouth :type Integer) (nose :type Integer))
  (bind _eye (Variables|Default|GetEye))
  (bind _mouth (Variables|Default|GetMouth))
  (bind _nose (Variables|Default|GetNose))
  (if bRandomize
    ;[1 1 1] Process to randomly change the part numbers of the face.
    (Variables|Default|SetnowEye (Math|Random|RandomInteger (Variables|Default|GetmaxEyeVolume)))
    (Variables|Default|SetnowMouth (Math|Random|RandomInteger (Variables|Default|GetmaxMouthVolume)))
    (Variables|Default|SetnowNose (Math|Random|RandomInteger (Variables|Default|GetmaxNoseVolume)))
    (else
      ;[1 1 1] Process to change each face part number to the one specified int the argument list.
      (Variables|Default|SetnowEye eye)
      (Variables|Default|SetnowMouth mouth)
      (Variables|Default|SetnowNose nose)))
  ;[1 1 1] Process to change the face parts.
  ;;[1 1 1] Process to  change the eye part based on the nowEye variable.
  (switch int (Variables|Default|GetnowEye)
    (:Default
      (Rendering|Material|SetMaterial _eye 0 "/Game/FaceTextures/M_TestEye3.M_TestEye3" :!label _label))
    (:0
      (Rendering|Material|SetMaterial _eye 0 "/Game/FaceTextures/M_TestEye1.M_TestEye1"))
    (:1
      (Rendering|Material|SetMaterial _eye 0 "/Game/FaceTextures/M_TestEye2.M_TestEye2"))
    (:2
      (goto _label)))
  ;;[1 1 1] Process to change the mouth part based on the nowMouth variable.
  (switch int (Variables|Default|GetnowMouth)
    (:Default
      (Rendering|Material|SetMaterial _mouth 0 "/Game/FaceTextures/M_TestMouth3.M_TestMouth3" :!label _label_2))
    (:0
      (Rendering|Material|SetMaterial _mouth 0 "/Game/FaceTextures/M_TestMouth1.M_TestMouth1"))
    (:1
      (Rendering|Material|SetMaterial _mouth 0 "/Game/FaceTextures/M_TestMouth2.M_TestMouth2"))
    (:2
      (goto _label_2)))
  ;;[1 1 1] Process to change the nose part based on the nowNose variable.
  (switch int (Variables|Default|GetnowNose)
    (:Default
      (Rendering|Material|SetMaterial _nose 0 "/Game/FaceTextures/M_TestNose3.M_TestNose3" :!label _label_3))
    (:0
      (Rendering|Material|SetMaterial _nose 0 "/Game/FaceTextures/M_TestNose1.M_TestNose1"))
    (:1
      (Rendering|Material|SetMaterial _nose 0 "/Game/FaceTextures/M_TestNose2.M_TestNose2"))
    (:2
      (goto _label_3))))